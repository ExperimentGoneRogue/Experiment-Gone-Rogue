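; BP_Donut is a donut actor with a randomized look and an Eat event.
; The construction script puts a dynamic instance of M_Donut on the mesh, picks chocolate, strawberry or caramel at random, then sets a random texture from that flavor's array.
; Eat only spawns a crumb particle effect at the actor's transform; it neither hides nor destroys the donut.
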(event Custom|Eat
  (bind _returnvalue (Transformation|GetActorTransform))
  (Effects|SpawnEmitteratLocation "/Game/P_Crumbs.P_Crumbs" (.location _returnvalue) (.rotation _returnvalue) (.scale _returnvalue)))

(event EventBeginPlay)

(event Collision|EventActorBeginOverlap
  (params (OtherActor :type Actor%20Object%20Reference)))

(event EventTick
  (params (DeltaSeconds :type Float%20%28single-precision%29)))

(fn ConstructionScript
  (bind _returnvalue (Rendering|Material|CreateDynamicMaterialInstance "/Game/M_Donut.M_Donut" "None" :!class /Script/Engine.KismetMaterialLibrary))
  (bind _output_get (Variables|Default|SetDynamicMaterial _returnvalue))
  (Rendering|Material|SetMaterial (Variables|Default|GetSM_Doughnut) 0 _output_get)
  (switch Utilities|FlowControl|Switch|SwitchoneDonutType (Utilities|Enum|ByteToEnumeDonutType (Math|Conversions|ToByte(Integer) (Math|Random|RandomIntegerinRange 0 2)))
    (:NewEnumerator0
      (Variables|Default|SetTexturesToUse (Variables|Default|GetChocolateTextures)))
    (:NewEnumerator1
      (Variables|Default|SetTexturesToUse (Variables|Default|GetStrawberryTextures)))
    (:NewEnumerator2
      (Variables|Default|SetTexturesToUse (Variables|Default|GetCaramelTextures))))
  (Rendering|Material|SetTextureParameterValue (Variables|Default|GetDynamicMaterial) "Texture" (Utilities|Array|Get(acopy) (Variables|Default|GetTexturesToUse) (Math|Random|RandomIntegerinRange 0 3))))